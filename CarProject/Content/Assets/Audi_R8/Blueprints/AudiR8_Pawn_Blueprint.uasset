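; Audi R8 car pawn with switchable lights and an orbit camera; this Blueprint holds no driving logic.
; Holding CarLights swaps two body material slots to emissive versions and shows four spotlights, and releasing it reverts both.
; Axis inputs yaw the spring arm, set its pitch within a clamp from its target rotation, and change arm length for zoom without limits.
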(event EventBeginPlay)

(event Collision|EventActorBeginOverlap
  (params (OtherActor :type Actor%20Object%20Reference)))

(event EventTick
  (params (DeltaSeconds :type Float%20%28single-precision%29)))

(event Input|ActionEvents|InputActionCarLights
  (params (Key :type Key%20Structure :default "None"))
  (bind _spotlight1 (Variables|Default|GetSpotLight1))
  (bind _spotlight2 (Variables|Default|GetSpotLight2))
  (bind _spotlight3 (Variables|Default|GetSpotLight3))
  (bind _spotlight4 (Variables|Default|GetSpotLight4))
  (bind _audi_r8 (Variables|Default|GetAudi_R8))
  (:Pressed
    (Rendering|Material|SetMaterial _audi_r8 5 "/Game/Assets/Audi_R8/white_lights_emissive_instance.white_lights_emissive_instance")
    (Rendering|Material|SetMaterial _audi_r8 6 "/Game/Assets/Audi_R8/red_lights_emissive_instance.red_lights_emissive_instance")
    (Rendering|SetVisibility _spotlight1 true false)
    (Rendering|SetVisibility _spotlight2 true false)
    (Rendering|SetVisibility _spotlight3 true false)
    (Rendering|SetVisibility _spotlight4 true false))
  (:Released
    (Rendering|Material|SetMaterial _audi_r8 5 "/Game/Assets/Audi_R8/white_lights_white_lights.white_lights")
    (Rendering|Material|SetMaterial _audi_r8 6 "/Game/Assets/Audi_R8/red_lights_red_lights.red_lights")
    (Rendering|SetVisibility _spotlight1 false false)
    (Rendering|SetVisibility _spotlight2 false false)
    (Rendering|SetVisibility _spotlight3 false false)
    (Rendering|SetVisibility _spotlight4 false false)))

(event Input|AxisEvents|InputAxisTurnAround
  (params (AxisValue :type Float%20%28single-precision%29))
  (Transformation|AddLocalRotation (Variables|Default|GetSpringArm) (Math|Rotator|MakeRotator 0.0 0.0 AxisValue) false false))

(event Input|AxisEvents|InputAxisLookup
  (params (AxisValue :type Float%20%28single-precision%29))
  (bind _springarm (Variables|Default|GetSpringArm))
  (bind _returnvalue (Class|SpringArmComponent|GetTargetRotation _springarm))
  (Transformation|SetRelativeRotation (Variables|Default|GetSpringArm) (Math|Rotator|MakeRotator 0.0 (Math|Float|Clamp(Float) (+ AxisValue (.pitch _returnvalue)) -75.0 75.0) (.yaw _returnvalue)) false false))

(event Input|AxisEvents|InputAxisZoomInOut
  (params (AxisValue :type Float%20%28single-precision%29))
  (bind _springarm (Variables|Default|GetSpringArm))
  (Variables|/Script/Engine.SpringArmComponent|SetTargetArmLength _springarm (+ AxisValue (Variables|/Script/Engine.SpringArmComponent|GetTargetArmLength _springarm))))

(fn ConstructionScript)